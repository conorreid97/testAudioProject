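; BP_Lich is an enemy that chases the player on sight and can be damaged and destroyed.
; A PawnSensing sighting of any pawn sets IsSeeingPlayer, which is never cleared here, and starts an AI move toward player character 0.
; HitEnemy sets Health to Damage minus Health (operands appear reversed), destroys the actor at zero or below, and prints debug text.
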(event OnSeePawn(PawnSensing)
  (params (Pawn :type Pawn%20Object%20Reference))
  (Variables|Default|SetisSeeingPlayer true)
  (CallFunction|FollowPlayer))

(event Custom|FollowPlayer
  (if (Variables|Default|GetisSeeingPlayer)
    (AI|AIMoveTo self "0, 0, 0" (Game|GetPlayerCharacter 0) 5.0 false)))

(event EventBeginPlay)

(event Collision|EventActorBeginOverlap
  (params (OtherActor :type Actor%20Object%20Reference)))

(event EventTick
  (params (DeltaSeconds :type Float%20%28single-precision%29)))

(event EventHitEnemy
  (params (Damage :type Float%20%28double-precision%29))
  (Development|PrintString "DAMAGE" true true "(R=1.000000,G=0.041057,B=0.678094,A=1.000000)")
  (bind _output_get (Variables|Default|SetHealth (- Damage (Variables|Default|GetHealth))))
  (if (<= _output_get 0.0)
    (Actor|DestroyActor)
    (else
      (Development|PrintString (Utilities|String|ToString(Float) _output_get)))))

(fn ConstructionScript)